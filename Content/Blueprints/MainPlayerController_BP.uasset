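; Player controller Blueprint that extends its parent's events for showing and hiding the store page and pause menu.
; After the parent shows the store page, it casts and caches the Store reference if needed, then calls that store's display function.
; The pause menu plays its move animation when shown and reverses it when removed, delaying briefly before hiding the widget and calling the parent's removal logic.
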(event `self.DisplayStorePage`
  (`parent.DisplayStorePage`)
  (`/Engine/EditorBlueprintResources/StandardMacros.IsValid` (`self.StoreRef`)
    (:`Is Valid`
      _)
    (:`Is Not Valid`
      (bind _asstore (cast `/Game/UI/Store` (`self.StorePage`)))
      (set `self.StoreRef` _asstore)))
  (`/Game/UI/Store.Controller_DisplayStorePage` (`self.StoreRef`)))

(event `self.RemoveStorePage`
  (`parent.RemoveStorePage`))

(event `self.DisplayPauseMenu`
  (`parent.DisplayPauseMenu`)
  (bind _aspause_menu (cast `/Game/UI/PauseMenu` (`self.PauseMenu`)))
  (`UserWidget.PlayAnimation` _aspause_menu (`/Game/UI/PauseMenu.MoveAnimation` _aspause_menu) 0.0 1 "Forward" 1.0 false))

(event `self.RemovePauseMenu`
  (bind _aspause_menu (cast `/Game/UI/PauseMenu` (`self.PauseMenu`)))
  (`UserWidget.PlayAnimation` _aspause_menu (`/Game/UI/PauseMenu.MoveAnimation` _aspause_menu) 0.0 1 "Reverse" 1.0 false)
  (`KismetSystemLibrary.Delay` 0.5)
  (`Widget.SetVisibility` (`self.PauseMenu`) "Hidden")
  (`parent.RemovePauseMenu`))

(fn `UserConstructionScript`)